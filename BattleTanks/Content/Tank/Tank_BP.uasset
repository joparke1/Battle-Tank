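; Tank_BP is the player-controlled tank pawn Blueprint, handling camera orbit and firing input.
; Azimuth and elevation axes rotate an AzimuthGimbal in yaw and the SpringArm in pitch, separating the two camera rotations.
; The Fire action calls Fire, and BeginPlay passes the TankBarrel and TankTurret components in through setter functions.
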(event EventBeginPlay
  (Class|Tank|SetBarrelReference (Variables|Default|GetTankBarrel))
  (Class|Tank|SetTurretReference (Variables|Default|GetTankTurret)))

(event Input|ActionEvents|InputActionFire
  (params (Key :type Key%20Structure))
  (:Pressed
    (Class|Tank|Fire)))

(event Input|AxisEvents|InputAxisAzimuthAxis
  (params (AxisValue :type Float%20%28single-precision%29))
  ;[1 1 1] Control Camera Rotation
  (Transformation|AddLocalRotation (Variables|Default|GetAzimuthGimbal) (Math|Rotator|MakeRotator 0.0 0.0 AxisValue) false false))

(event Input|AxisEvents|InputAxisElevationAxis
  (params (AxisValue :type Float%20%28single-precision%29))
  ;[1 1 1] Control Camera Rotation
  (Transformation|AddLocalRotation (Variables|Default|GetSpringArm) (Math|Rotator|MakeRotator 0.0 AxisValue 0.0) false false))

(fn ConstructionScript)